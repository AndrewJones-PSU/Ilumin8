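; ICP_Instance is a global Blueprint that manages the InitializeConnection and MainPanel widgets and streams commands to an Arduino.
; Show events create each widget once and cache it for reuse, while hide events remove it from its parent.
; Initialize caps the frame rate, disables VSync and starts a looping timer at a matching 80 Hz.
; Each tick writes a command byte, the length and the buffered DataStream, then clears the buffer and resets RecursionCounter.
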(event `ShowInitializeConnection`
  ;[0.9688 1 0] Show and Hide the InitializeConnection Widget
  (`/Engine/EditorBlueprintResources/StandardMacros.IsValid` (`self.InitializeConnectionWidget`)
    (:`Is Valid`
      _)
    (:`Is Not Valid`
      (bind _returnvalue (`|CreateWidget` "/Game/Widgets/InitializeConnection.InitializeConnection_C"))
      (bind _output_get (set `self.InitializeConnectionWidget` _returnvalue))))
  (`UserWidget.AddToViewport` _output_get 0))

(event `HideInitializeConnection`
  (bind _initializeconnectionwidget (`self.InitializeConnectionWidget`))
  ;[0.9688 1 0] Show and Hide the InitializeConnection Widget
  (`/Engine/EditorBlueprintResources/StandardMacros.IsValid` _initializeconnectionwidget
    (:`Is Valid`
      (`Widget.RemoveFromParent` _initializeconnectionwidget))))

(event `ShowMainPanel`
  ;[0 1 0.8125] Show and Hide the MainPanel Widget
  (`/Engine/EditorBlueprintResources/StandardMacros.IsValid` (`self.MainPanelWidget`)
    (:`Is Valid`
      _)
    (:`Is Not Valid`
      (bind _returnvalue (`|CreateWidget` "/Game/Widgets/MainPanel.MainPanel_C"))
      (bind _output_get (set `self.MainPanelWidget` _returnvalue))))
  (`UserWidget.AddToViewport` _output_get 0))

(event `Initialize`
  ;[1 0 0.9375] Initialize our Send Datastream Function and set to use 80FPS
  (`KismetSystemLibrary.ExecuteConsoleCommand` "t.MaxFPS 80" null)
  (`KismetSystemLibrary.ExecuteConsoleCommand` "r.VSync false" null)
  (bind _returnvalue (`KismetSystemLibrary.K2_SetTimerDelegate` (delegate `SendDatastream`) 0.0125 true))
  (set `self.DatastreamTimer` _returnvalue))

(event `HideMainPanel`
  (bind _mainpanelwidget (`self.MainPanelWidget`))
  ;[0 1 0.8125] Show and Hide the MainPanel Widget
  (`/Engine/EditorBlueprintResources/StandardMacros.IsValid` _mainpanelwidget
    (:`Is Valid`
      (`Widget.RemoveFromParent` _mainpanelwidget))))

(event `SendDatastream`
  (bind _arduino (`self.Arduino`))
  (bind _datastream (`self.DataStream`))
  ;[0.6172 0 1] Sends a Datastream of commands to the arduino
  (`Serial.WriteByte` _arduino (enumliteral `/Game/Blueprints/Global/SerialCommands` "NewEnumerator2"))
  (`Serial.WriteByte` _arduino (`KismetMathLibrary.Conv_IntToByte` (`KismetArrayLibrary.Array_Length` (`self.DataStream`))))
  (`Serial.WriteBytes` _arduino _datastream)
  (`KismetArrayLibrary.Array_Clear` _datastream)
  (set `self.RecursionCounter` 0))